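; Core Game Instance that keeps RPG party, inventory, global variables and player field position data across levels.
; On Init it seeds each party member's state at level 1 from their initial max HP and MP.
; Interface calls store battle-updated states and the last field transform, tagged with level name and area info from the GameMode.
; Interface getters expose this data, including party members filtered to those not knocked out.
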(event `self.ReceiveInit`
  (for _array_element (`self.PartyMembers`)
    (bind (_maxhp _maxmp) (break `/Game/Definitions/Structs/S_CharAttributes` (`/Game/Data/DataAssets/BattleCharData/PDA_BattleCharData.InitialAttributes` (`/Game/Data/DataAssets/PartyMemberData/PDA_PartyMemberData.BattleCharData` _array_element))))
    (`KismetArrayLibrary.Array_Add` (`self.PartyStates`) (make `/Game/Definitions/Structs/S_CharState` _maxhp _maxmp 1))))

(event `/Game/Definitions/Interfaces/BPI_InstanceStorage.I_StoreFieldPosition`
  (params (LastFieldTransform :type "Transform Structure"))
  (`self.StoreFieldPosition` LastFieldTransform))

(event `/Game/Definitions/Interfaces/BPI_InstanceStorage.I_StorePartyStates`
  (params (PartyMembers :type "Array of /Game/Blueprints/Battle/BattleChars/BP_BattleChar_BASE Object Reference (by ref)"))
  (`self.StorePartyStates` PartyMembers))

(fn `GetAlivePartyMembers`
  (returns (AliveMembers :type "Array of /Game/Data/DataAssets/PartyMemberData/PDA_PartyMemberData Object Reference"))
  (locals (Members :type "Array of /Game/Data/DataAssets/PartyMemberData/PDA_PartyMemberData Object Reference"))
  (for (_array_element _array_index) (`self.PartyStates`)
    (if (not (`.IsKnockedOut_14_79D64E03441BDE08E6B41AAA1ED458F3` (break `/Game/Definitions/Structs/S_CharState` _array_element)))
      (`KismetArrayLibrary.Array_Add` (`local.Members`) (`|GetArrayItem` (`self.PartyMembers`) _array_index))))
  (return (`local.Members`)))

(fn `I_GetAlivePartyMembers`
  (returns (AliveMembers :type "Array of /Game/Data/DataAssets/PartyMemberData/PDA_PartyMemberData Object Reference"))
  (bind _alivemembers (`self.GetAlivePartyMembers`))
  (return _alivemembers))

(fn `I_GetGlobalVariables`
  (returns (GlobalVriables :type "/Game/Data/DataAssets/GlobalVariables/PDA_GlobalVariables Object Reference"))
  (return (`self.GlobalVariables`)))

(fn `I_GetInventory`
  (returns (Inventory :type "Map of /Game/Data/DataAssets/ItemData/PDA_ItemData Object Reference to Integer"))
  (return (`self.Inventory`)))

(fn `I_GetPartyMembers`
  (returns (PartyMembers :type "Array of /Game/Data/DataAssets/PartyMemberData/PDA_PartyMemberData Object Reference"))
  (return (`self.PartyMembers`)))

(fn `I_GetPartyStates`
  (returns (States :type "Array of /Game/Definitions/Structs/S_CharState Structure"))
  (return (`self.PartyStates`)))

(fn `I_GetPlayerFieldPosition`
  (returns (PlayerFieldPosition :type "/Game/Definitions/Structs/S_FieldPosition Structure"))
  (return (`self.PlayerFieldPosition`)))

(fn `StoreFieldPosition`
  (params (LastFieldTransform :type "Transform Structure"))
  (setmembers `/Game/Definitions/Structs/S_FieldPosition` :`StructRef` (`self.PlayerFieldPosition`) :`LastFieldTransform` LastFieldTransform)
  (bind _areadata (message `/Game/Definitions/Interfaces/BPI_AreaControl.I_GetCurrentAreaData` (`GameplayStatics.GetGameMode`)))
  (bind _returnvalue (`GameplayStatics.GetCurrentLevelName` true))
  (setmembers `/Game/Definitions/Structs/S_FieldPosition` :`StructRef` (`self.PlayerFieldPosition`) :`FieldLevelName` _returnvalue :`AreaInfo` _areadata))

(fn `StorePartyStates`
  (params (PartyMembers :type "Array of /Game/Blueprints/Battle/BattleChars/BP_BattleChar_BASE Object Reference"))
  (for (_array_element _array_index) PartyMembers
    (`KismetArrayLibrary.Array_Set` (`self.PartyStates`) _array_index (`/Game/Blueprints/Components/AC_BattleStats.State` (`/Game/Blueprints/Battle/BattleChars/BP_BattleChar_BASE.AC_BattleStats` _array_element)) true)))