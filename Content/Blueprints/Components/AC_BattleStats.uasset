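; Battle stats component that holds a character's attributes and HP, MP, XP, level and knockout state.
; Skill-calculated damage, reduced by capped percentage defense and defending, or healing updates HP, health bar and combat numbers, triggering shake or knockout on damage.
; GainXP recursively carries surplus XP across level-ups using a global table.
; Restoring saved state rebuilds attributes from cumulative per-level bonuses and reapplies the knockout animation.
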(fn `ApplyAttributes`
  (locals (LoopAttributes :type "/Game/Definitions/Structs/S_CharAttributes Structure"))
  (for _index (range (+ (- (`.Level_7_7BFB54774843A21061AEC381EECE1E30` (break `/Game/Definitions/Structs/S_CharState` (`self.State`))) 2) 1))
    (set `local.LoopAttributes` (`|GetArrayItem` (`/Game/Data/DataAssets/BattleCharData/PDA_BattleCharData.LevelAttributes` (`/Game/Blueprints/Battle/BattleChars/BP_BattleChar_BASE.BattleCharData` (`self.OwningBattleChar`))) _index))
    (`|ExecutionSequence`
      (:`then_0`
        (setmembers `/Game/Definitions/Structs/S_CharAttributes` :`StructRef` (`self.Attributes`) :`MaxHP` (+ (`.MaxHP_2_9D9D02EB4B6A9CDA3DBD53B1E7749C14` (break `/Game/Definitions/Structs/S_CharAttributes` (`self.Attributes`))) (`.MaxHP_2_9D9D02EB4B6A9CDA3DBD53B1E7749C14` (break `/Game/Definitions/Structs/S_CharAttributes` (`local.LoopAttributes`))))))
      (:`then_1`
        (setmembers `/Game/Definitions/Structs/S_CharAttributes` :`StructRef` (`self.Attributes`) :`MaxMP` (+ (`.MaxMP_4_550DD8344CE1CB179CF3CAB27F972FED` (break `/Game/Definitions/Structs/S_CharAttributes` (`self.Attributes`))) (`.MaxMP_4_550DD8344CE1CB179CF3CAB27F972FED` (break `/Game/Definitions/Structs/S_CharAttributes` (`local.LoopAttributes`))))))
      (:`then_2`
        (setmembers `/Game/Definitions/Structs/S_CharAttributes` :`StructRef` (`self.Attributes`) :`AttackPower` (+ (`.AttackPower_10_2E44E3C04839B436F2103E9068ACB211` (break `/Game/Definitions/Structs/S_CharAttributes` (`self.Attributes`))) (`.AttackPower_10_2E44E3C04839B436F2103E9068ACB211` (break `/Game/Definitions/Structs/S_CharAttributes` (`local.LoopAttributes`))))))
      (:`then_3`
        (setmembers `/Game/Definitions/Structs/S_CharAttributes` :`StructRef` (`self.Attributes`) :`SpellPower` (+ (`.SpellPower_11_EBDFED4547783C2E2943DABFAE4760A8` (break `/Game/Definitions/Structs/S_CharAttributes` (`self.Attributes`))) (`.SpellPower_11_EBDFED4547783C2E2943DABFAE4760A8` (break `/Game/Definitions/Structs/S_CharAttributes` (`local.LoopAttributes`))))))
      (:`then_4`
        (setmembers `/Game/Definitions/Structs/S_CharAttributes` :`StructRef` (`self.Attributes`) :`PhysDefense` (+ (`.PhysDefense_13_57347AC64749E4808138709F378BC5C9` (break `/Game/Definitions/Structs/S_CharAttributes` (`self.Attributes`))) (`.PhysDefense_13_57347AC64749E4808138709F378BC5C9` (break `/Game/Definitions/Structs/S_CharAttributes` (`local.LoopAttributes`))))))
      (:`then_5`
        (setmembers `/Game/Definitions/Structs/S_CharAttributes` :`StructRef` (`self.Attributes`) :`SpellDefense` (+ (`.SpellDefense_15_01B1220246096398BFC0BF8BBB7CEF5B` (break `/Game/Definitions/Structs/S_CharAttributes` (`self.Attributes`))) (`.SpellDefense_15_01B1220246096398BFC0BF8BBB7CEF5B` (break `/Game/Definitions/Structs/S_CharAttributes` (`local.LoopAttributes`))))))
      (:`then_6`
        (setmembers `/Game/Definitions/Structs/S_CharAttributes` :`StructRef` (`self.Attributes`) :`CritChance` (+ (`.CritChance_17_EA3D31904087A938DC9120BB07742B41` (break `/Game/Definitions/Structs/S_CharAttributes` (`self.Attributes`))) (`.CritChance_17_EA3D31904087A938DC9120BB07742B41` (break `/Game/Definitions/Structs/S_CharAttributes` (`local.LoopAttributes`)))))))))

(fn `DamageAfterDefense`
  (params (IncomingDamage :type "Float (double-precision)") (IsPhysical :type Boolean))
  (returns (Damage :type "Float (double-precision)"))
  (bind _globalvariables (`/Game/Definitions/FunctionLibraries/BPFL_CORE.GetGlobalVariables`))
  (bind ((`PhysDefense_13_57347AC64749E4808138709F378BC5C9` _physdefense) (`SpellDefense_15_01B1220246096398BFC0BF8BBB7CEF5B` _spelldefense)) (break `/Game/Definitions/Structs/S_CharAttributes` (`self.Attributes`)))
  (return (* (- IncomingDamage (* (`local.IncomingDamage`) (/ (`KismetMathLibrary.FMin` (/ (select `bool` (`local.IsPhysical`) :`false` _spelldefense :`true` _physdefense) (`/Game/Data/DataAssets/GlobalVariables/PDA_GlobalVariables.DefensiveScaleDivider` _globalvariables)) (`/Game/Data/DataAssets/GlobalVariables/PDA_GlobalVariables.MaxDefensePercentage` _globalvariables)) 100.0))) (select `bool` (`/Game/Blueprints/Battle/BattleChars/BP_BattleChar_BASE.IsDefending` (`self.OwningBattleChar`)) :`false` 1.0 :`true` (`/Game/Data/DataAssets/GlobalVariables/PDA_GlobalVariables.DefendMultiplier` (`/Game/Definitions/FunctionLibraries/BPFL_CORE.GetGlobalVariables`))))))

(fn `GainXP`
  (params (Amount :type Integer))
  (locals (XPToLevelUp :type Integer) (RemainingXP :type Integer) (NewXP :type Integer))
  (if (`KismetArrayLibrary.Array_IsValidIndex` (`/Game/Data/DataAssets/GlobalVariables/PDA_GlobalVariables.LevelXP` (`/Game/Definitions/FunctionLibraries/BPFL_CORE.GetGlobalVariables`)) (`.Level_7_7BFB54774843A21061AEC381EECE1E30` (break `/Game/Definitions/Structs/S_CharState` (`self.State`))))
    (set `local.NewXP` (+ (`local.Amount`) (`.XP_15_B5968CD64269F7D35BAFE68E1D27D8C0` (break `/Game/Definitions/Structs/S_CharState` (`self.State`)))))
    (set `local.XPToLevelUp` (`|GetArrayItem` (`/Game/Data/DataAssets/GlobalVariables/PDA_GlobalVariables.LevelXP` (`/Game/Definitions/FunctionLibraries/BPFL_CORE.GetGlobalVariables`)) (`.Level_7_7BFB54774843A21061AEC381EECE1E30` (break `/Game/Definitions/Structs/S_CharState` (`self.State`)))))
    (if (>= (`local.NewXP`) (`local.XPToLevelUp`))
      (set `local.RemainingXP` (- (`local.NewXP`) (`local.XPToLevelUp`)))
      (setmembers `/Game/Definitions/Structs/S_CharState` :`StructRef` (`self.State`) :`Level` (`KismetMathLibrary.Min` (+ (`.Level_7_7BFB54774843A21061AEC381EECE1E30` (break `/Game/Definitions/Structs/S_CharState` (`self.State`))) 1) (`KismetArrayLibrary.Array_Length` (`/Game/Data/DataAssets/GlobalVariables/PDA_GlobalVariables.LevelXP` (`/Game/Definitions/FunctionLibraries/BPFL_CORE.GetGlobalVariables`)))) :`XP` 0)
      (`self.GainXP` (`local.RemainingXP`))
      (else
        (setmembers `/Game/Definitions/Structs/S_CharState` :`StructRef` (`self.State`) :`XP` (`local.NewXP`))
        (return)))
    (else
      (return))))

(fn `Initialize`
  (params (OwningBattleChar :type "/Game/Blueprints/Battle/BattleChars/BP_BattleChar_BASE Object Reference"))
  (bind (_maxhp _maxmp) (break `/Game/Definitions/Structs/S_CharAttributes` (`self.Attributes`)))
  (set `self.OwningBattleChar` OwningBattleChar)
  (set `self.Attributes` (`/Game/Data/DataAssets/BattleCharData/PDA_BattleCharData.InitialAttributes` (`/Game/Blueprints/Battle/BattleChars/BP_BattleChar_BASE.BattleCharData` (`self.OwningBattleChar`))))
  (setmembers `/Game/Definitions/Structs/S_CharState` :`StructRef` (`self.State`) :`HP` _maxhp :`MP` _maxmp))

(fn `OverrideStateFromSaved`
  (params (State :type "/Game/Definitions/Structs/S_CharState Structure"))
  (set `self.State` State)
  (`self.ApplyAttributes`)
  (if (`.IsKnockedOut_14_79D64E03441BDE08E6B41AAA1ED458F3` (break `/Game/Definitions/Structs/S_CharState` (`self.State`)))
    (`/Game/Blueprints/Battle/BattleChars/BP_BattleChar_BASE.ForceKnockoutAnim` (`self.OwningBattleChar`))))

(fn `ReceiveDamageEffect`
  (params (InstigatorStats :type "/Game/Blueprints/Components/AC_BattleStats Object Reference") (SkillData :type "/Game/Data/DataAssets/SkillData/PDA_SkillData Object Reference"))
  (locals (FinalValue :type "Float (double-precision)" :default 0.0) (IsCritical :type Boolean :default false))
  (`|ExecutionSequence`
    (:`then_0`
      (bind (_calculatedpower _wascritical) (`/Game/Data/DataAssets/SkillData/PDA_SkillData.GetCalculatedPower` (`local.SkillData`) (`local.InstigatorStats`)))
      (set `local.IsCritical` _wascritical)
      (bind _damage (`self.DamageAfterDefense` _calculatedpower (`/Game/Data/DataAssets/SkillData/PDA_SkillData.IsPhysical` (`local.SkillData`))))
      (set `local.FinalValue` (`KismetMathLibrary.Conv_IntToDouble` (`KismetMathLibrary.Max` (`KismetMathLibrary.Round` _damage) 1)))
      (setmembers `/Game/Definitions/Structs/S_CharState` :`StructRef` (`self.State`) :`HP` (`KismetMathLibrary.FMax` (- (`.HP_2_C369CE804EF5F54AA33FDF841CB664C7` (break `/Game/Definitions/Structs/S_CharState` (`self.State`))) (`local.FinalValue`))))
      (bind _widgethealthmana (`/Game/Blueprints/Battle/BattleChars/BP_BattleChar_BASE.WidgetHealthMana` (`self.OwningBattleChar`))
        (:`then`
          (`/Game/UI/Widgets/Battle/WBP_BattleHealthMana.UpdateHP` _widgethealthmana (`.HP_2_C369CE804EF5F54AA33FDF841CB664C7` (break `/Game/Definitions/Structs/S_CharState` (`self.State`))) (`.MaxHP_2_9D9D02EB4B6A9CDA3DBD53B1E7749C14` (break `/Game/Definitions/Structs/S_CharAttributes` (`self.Attributes`)))))
        (:`else`)))
    (:`then_1`
      (`/Game/UI/Widgets/Battle/WBP_CombatText.ShowText` (`/Game/Blueprints/Battle/BattleChars/BP_BattleChar_BASE.WidgetCombatNumber` (`self.OwningBattleChar`)) (`local.FinalValue`) (select `bool` (`local.IsCritical`) :`false` "NewEnumerator0" :`true` "NewEnumerator1" :!type "/Game/Definitions/Enums/E_CombatTextType Enum")))
    (:`then_2`
      (if (<= (`.HP_2_C369CE804EF5F54AA33FDF841CB664C7` (break `/Game/Definitions/Structs/S_CharState` (`self.State`))) 0.0)
        (setmembers `/Game/Definitions/Structs/S_CharState` :`StructRef` (`self.State`) :`IsKnockedOut` true)
        (`/Game/Blueprints/Battle/BattleChars/BP_BattleChar_BASE.DepletedHealth` (`self.OwningBattleChar`))
        (else
          (`/Game/Blueprints/Components/AC_Shaker.StartShake` (`/Game/Blueprints/Battle/BattleChars/BP_BattleChar_BASE.AC_Shaker` (`self.OwningBattleChar`))))))))

(fn `ReceiveHealEffect`
  (params (InstigatorStats :type "/Game/Blueprints/Components/AC_BattleStats Object Reference") (SkillData :type "/Game/Data/DataAssets/SkillData/PDA_SkillData Object Reference"))
  (locals (FinalValue :type "Float (double-precision)" :default 0.0) (IsCritical :type Boolean :default false))
  (`|ExecutionSequence`
    (:`then_0`
      (bind (_calculatedpower _wascritical) (`/Game/Data/DataAssets/SkillData/PDA_SkillData.GetCalculatedPower` (`local.SkillData`) (`local.InstigatorStats`)))
      (set `local.IsCritical` _wascritical)
      (set `local.FinalValue` (`KismetMathLibrary.Conv_IntToDouble` (`KismetMathLibrary.Max` (`KismetMathLibrary.Round` _calculatedpower) 1)))
      (setmembers `/Game/Definitions/Structs/S_CharState` :`StructRef` (`self.State`) :`HP` (`KismetMathLibrary.FMin` (+ (`.HP_2_C369CE804EF5F54AA33FDF841CB664C7` (break `/Game/Definitions/Structs/S_CharState` (`self.State`))) (`local.FinalValue`)) (`.MaxHP_2_9D9D02EB4B6A9CDA3DBD53B1E7749C14` (break `/Game/Definitions/Structs/S_CharAttributes` (`self.Attributes`)))))
      (bind _widgethealthmana (`/Game/Blueprints/Battle/BattleChars/BP_BattleChar_BASE.WidgetHealthMana` (`self.OwningBattleChar`))
        (:`then`
          (`/Game/UI/Widgets/Battle/WBP_BattleHealthMana.UpdateHP` _widgethealthmana (`.HP_2_C369CE804EF5F54AA33FDF841CB664C7` (break `/Game/Definitions/Structs/S_CharState` (`self.State`))) (`.MaxHP_2_9D9D02EB4B6A9CDA3DBD53B1E7749C14` (break `/Game/Definitions/Structs/S_CharAttributes` (`self.Attributes`)))))
        (:`else`)))
    (:`then_1`
      (`/Game/UI/Widgets/Battle/WBP_CombatText.ShowText` (`/Game/Blueprints/Battle/BattleChars/BP_BattleChar_BASE.WidgetCombatNumber` (`self.OwningBattleChar`)) (`local.FinalValue`) (select `bool` (`local.IsCritical`) :`false` "NewEnumerator2" :`true` "NewEnumerator1" :!type "/Game/Definitions/Enums/E_CombatTextType Enum")))))

(fn `UpdateMana`
  (params (ChangeAmount :type "Float (double-precision)"))
  (setmembers `/Game/Definitions/Structs/S_CharState` :`StructRef` (`self.State`) :`MP` (`KismetMathLibrary.FClamp` (+ (`local.ChangeAmount`) (`.MP_4_A03A797841E5C9154D8588A6FCE9EFC9` (break `/Game/Definitions/Structs/S_CharState` (`self.State`)))) 0.0 (`.MaxMP_4_550DD8344CE1CB179CF3CAB27F972FED` (break `/Game/Definitions/Structs/S_CharAttributes` (`self.Attributes`)))))
  (bind _widgethealthmana (`/Game/Blueprints/Battle/BattleChars/BP_BattleChar_BASE.WidgetHealthMana` (`self.OwningBattleChar`))
    (:`then`
      (`/Game/UI/Widgets/Battle/WBP_BattleHealthMana.UpdateMP` _widgethealthmana (`.MP_4_A03A797841E5C9154D8588A6FCE9EFC9` (break `/Game/Definitions/Structs/S_CharState` (`self.State`))) (`.MaxMP_4_550DD8344CE1CB179CF3CAB27F972FED` (break `/Game/Definitions/Structs/S_CharAttributes` (`self.Attributes`)))))
    (:`else`)))