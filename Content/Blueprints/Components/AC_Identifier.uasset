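; AC_Identifier is an actor component that records whether its owner's ID has been triggered and restores that state when play begins.
; TriggerID reads the owner's ID through an interface message and adds it to the triggered IDs on the Game Instance.
; On BeginPlay, ApplyTriggered asks the Game Instance whether that ID is already triggered and, if so, sends the owner a force-interact message.
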(event `self.ReceiveBeginPlay`
  (`self.ApplyTriggered`))

(fn `ApplyTriggered`
  (bind _id (message `/Game/Definitions/Interfaces/BPI_Interactable.I_GetID` (`self.GetOwner`)))
  (bind _value (message `/Game/Definitions/Interfaces/BPI_InstanceStorage.I_IsIDTriggered` (`GameplayStatics.GetGameInstance`) _id))
  (if _value
    (message `/Game/Definitions/Interfaces/BPI_Interactable.I_ForceInteract` (`self.GetOwner`))))

(fn `TriggerID`
  (bind _id (message `/Game/Definitions/Interfaces/BPI_Interactable.I_GetID` (`self.GetOwner`)))
  (message `/Game/Definitions/Interfaces/BPI_InstanceStorage.I_AddTriggeredID` (`GameplayStatics.GetGameInstance`) _id))