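; Base actor for battle characters, party members or otherwise, with a sprite, stats component, target pointer, combat text and portrait/health widgets.
; Received skill effects go to ACBattleStats and spawn particles at head, middle or feet, while outgoing effects route through BattleManager.
; Attacks play an override animation or fall back to a timeline hop.
; Depleted health updates team status, then party members jump to a downed state and others slide out and hide.
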(event `self.ReceiveBeginPlay`
  (`|ExecutionSequence`
    (:`then_0`
      (set `self.SpawnedLocation` (`self.K2_GetActorLocation`))
      (bind _aswbp_target_pointer (cast `/Game/UI/Widgets/WBP_TargetPointer` (`WidgetComponent.GetUserWidgetObject` (`self.WidgetPointer`))))
      (set `self.WidgetTargetPointer` _aswbp_target_pointer)
      (bind _aswbp_combat_text (cast `/Game/UI/Widgets/Battle/WBP_CombatText` (`WidgetComponent.GetUserWidgetObject` (`self.WidgetCombatText`))))
      (set `self.WidgetCombatNumber` _aswbp_combat_text))
    (:`then_1`
      (`/Game/Blueprints/Components/AC_Shaker.Initialize` (`self.AC_Shaker`) (`self.Sprite`))
      (`/Game/Blueprints/Components/AC_BattleStats.Initialize` (`self.AC_BattleStats`) self))
    (:`then_2`
      (bind _returnvalue (`PrimitiveComponent.CreateDynamicMaterialInstance` (`self.Sprite`) 0 null "None"))
      (set `self.DynamicSpriteMat` _returnvalue))))

(event `PlayAttackAnim`
  (bind (_spawnedlocation_x _spawnedlocation_y _spawnedlocation_z) (`KismetMathLibrary.BreakVector` (`self.SpawnedLocation`)))
  (bind _attackanimdefault (`/Game/Data/DataAssets/BattleCharData/PDA_BattleCharData.AttackAnimDefault` (`self.BattleCharData`))
    (:`then`
      (`PaperZDPlaySlotOverrideAction.PlayAnimationOverrideWithCallbacks` (`PaperZDAnimationComponent.AnimInstance` (`self.AnimationComponent`)) _attackanimdefault
        (:`OnCompleted`
          _)
        (:`OnCancelled`
          _))
      (`KismetSystemLibrary.RetriggerableDelay` (`/Game/Data/DataAssets/GlobalVariables/PDA_GlobalVariables.DelayAfterAttackAnim` (`/Game/Definitions/FunctionLibraries/BPFL_CORE.GetGlobalVariables`)))
      (`/Game/Blueprints/Battle/BP_BattleManager.MoveBackFromActive` (`self.BattleManager`)))
    (:`else`
      (`TimelineComponent.SetPlayRate` (`self.AnimDoubleJump`) (`self.JumpPlayRate`))
      (bind (_direction _alpha) (`Timeline|AnimDoubleJump` :!via `PlayFromStart`)
        (:`Update`
          (`self.K2_SetActorLocation` (`KismetMathLibrary.MakeVector` _spawnedlocation_x _spawnedlocation_y (+ _spawnedlocation_z (* _alpha (`self.JumpHeight`))))))
        (:`Finished`
          (`/Game/Blueprints/Battle/BP_BattleManager.FinishedTimelineAttackAnim` (`self.BattleManager`)))))))

(event `PlayKnockoutAnim`
  (`TimelineComponent.SetPlayRate` (`self.AnimKnockout`) (`self.KnockoutAnimPlayRate`))
  (bind (_direction _alpha) (`Timeline|AnimKnockout` :!via `PlayFromStart`)
    (:`Update`
      (`self.K2_SetActorLocation` (`KismetMathLibrary.VLerp` (`self.SpawnedLocation`) (+ (`self.SpawnedLocation`) (`self.KnockoutOffset`)) _alpha)))
    (:`Finished`
      (`self.SetActorHiddenInGame` true))))

(fn `AssignBattleHealthManaWidget`
  (params (WidgetHealthMana :type "/Game/UI/Widgets/Battle/WBP_BattleHealthMana Object Reference"))
  (bind (_maxhp _maxmp) (break `/Game/Definitions/Structs/S_CharAttributes` (`/Game/Blueprints/Components/AC_BattleStats.Attributes` (`self.AC_BattleStats`))))
  (bind (_hp _mp) (break `/Game/Definitions/Structs/S_CharState` (`/Game/Blueprints/Components/AC_BattleStats.State` (`self.AC_BattleStats`))))
  (set `self.WidgetHealthMana` WidgetHealthMana)
  (`/Game/UI/Widgets/Battle/WBP_BattleHealthMana.Activate` (`self.WidgetHealthMana`) (`/Game/Data/DataAssets/BattleCharData/PDA_BattleCharData.DisplayName` (`self.BattleCharData`)) _maxhp _hp _maxmp _mp))

(fn `DepletedHealth`
  (`|ExecutionSequence`
    (:`then_0`
      (`/Game/Blueprints/Battle/BP_BattleManager.UpdateTeamAlive` (`self.BattleManager`) self)
      (bind _widgetportrait (`self.WidgetPortrait`)
        (:`then`
          (`/Game/UI/Widgets/Battle/WBP_Portrait.HidePortrait` _widgetportrait))
        (:`else`)))
    (:`then_1`
      (if (`self.IsPartyMember`)
        (`PaperZDAnimInstance.JumpToNode` (`PaperZDAnimationComponent.AnimInstance` (`self.AnimationComponent`)) "JumpDowned" "None")
        (else
          (`self.PlayKnockoutAnim`))))))

(fn `ExecuteBattleEffect`
  (`/Game/Blueprints/Battle/BP_BattleManager.ApplyBattleEffect` (`self.BattleManager`) (`self.AC_BattleStats`)))

(fn `GetSkillByIndex`
  (params (Index :type Integer))
  (returns (SkillData :type "/Game/Data/DataAssets/SkillData/PDA_SkillData Object Reference"))
  (if (<= Index -1)
    (return (`/Game/Data/DataAssets/BattleCharData/PDA_BattleCharData.BasicAttackData` (`self.BattleCharData`)))
    (else
      (return (`|GetArrayItem` (`/Game/Data/DataAssets/BattleCharData/PDA_BattleCharData.Skills` (`self.BattleCharData`)) (`local.Index`))))))

(fn `HideBattlePortrait`
  (bind _widgetportrait (`self.WidgetPortrait`)
    (:`then`
      (`/Game/UI/Widgets/Battle/WBP_Portrait.HidePortrait` _widgetportrait)
      (set `self.WidgetPortrait` null))
    (:`else`)))

(fn `ReceiveBattleEffect`
  (params (InstigatorStats :type "/Game/Blueprints/Components/AC_BattleStats Object Reference") (SkillData :type "/Game/Data/DataAssets/SkillData/PDA_SkillData Object Reference"))
  (`/Game/Blueprints/Components/AC_BattleStats.ReceivedBattleEffect` (`self.AC_BattleStats`) InstigatorStats SkillData)
  (`NiagaraFunctionLibrary.SpawnSystemAtLocation` (`/Game/Data/DataAssets/SkillData/PDA_SkillData.ParticleEffect` (`local.SkillData`)) (`SceneComponent.K2_GetComponentLocation` (select `/Game/Definitions/Enums/E_TargetPosition` (`/Game/Data/DataAssets/SkillData/PDA_SkillData.ParticlePosition` (`local.SkillData`)) :`NewEnumerator0` (`self.Loc_Head`) :`NewEnumerator1` (`self.Loc_Middle`) :`NewEnumerator2` (`self.Loc_Feet`))) (struct :`Yaw` 180.0) (1.0 1.0 1.0) true true "AutoRelease"))

(fn `SetDefending`
  (params (SetActive :type Boolean))
  (set `self.IsDefending` SetActive))

(fn `SetPointerVisibility`
  (params (SetVisible :type Boolean))
  (if SetVisible
    (`/Game/UI/Widgets/WBP_TargetPointer.ShowPointer` (`self.WidgetTargetPointer`))
    (`MaterialInstanceDynamic.SetScalarParameterValue` (`self.DynamicSpriteMat`) "IsPulsing" 1.0)
    (else
      (`/Game/UI/Widgets/WBP_TargetPointer.HidePointer` (`self.WidgetTargetPointer`))
      (`MaterialInstanceDynamic.SetScalarParameterValue` (`self.DynamicSpriteMat`) "IsPulsing" 0.0))))

(fn `UserConstructionScript`)