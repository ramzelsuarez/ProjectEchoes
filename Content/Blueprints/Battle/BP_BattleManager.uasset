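; Battle manager pawn that runs turn-based party combat, from spawning both teams to returning to the field level.
; Turns follow a party-then-enemies queue, rebuilt when empty; enemies use basic attacks on party targets.
; Players choose via the action menu, then aim with Enhanced Input once the manager is possessed.
; It also handles deaths, fleeing and results, with timeline-driven character moves, camera sway and chromatic pulses.
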(event `self.ReceiveBeginPlay`
  (message `/Game/Definitions/Interfaces/BPI_UIControl.I_InitWidgetBattle` (`GameplayStatics.GetPlayerController` 0))
  (`self.StartBattle`))

(event `self.ReceivePossessed`
  (params (NewController :type "Controller Object Reference"))
  (bind _asplayer_controller (cast `PlayerController` (`self.GetController`)))
  (`EnhancedInputSubsystemInterface.AddMappingContext` (pcsubsystem `EnhancedInputLocalPlayerSubsystem` _asplayer_controller) "/Game/Inputs/BattleNav/IMC_BattleNav.IMC_BattleNav" 0 (struct)))

(event `StartCameraSway`
  (bind (_relativerotation_roll _relativerotation_pitch) (`KismetMathLibrary.BreakRotator` (`SceneComponent.RelativeRotation` (`self.Camera`))))
  (`TimelineComponent.SetPlayRate` (`self.AnimCameraSway`) (`self.CameraSwayRate`))
  (bind (_direction _yawrotation) (`Timeline|AnimCameraSway`)
    (:`Update`
      (`SceneComponent.K2_SetRelativeRotation` (`self.Camera`) (`KismetMathLibrary.MakeRotator` _relativerotation_roll _relativerotation_pitch (* _yawrotation (`self.CameraSwayDistance`))) false false))))

(event `PlayChromaticPulse`
  (`TimelineComponent.SetPlayRate` (`self.AnimChromatic`) (`self.ChromaticPlayRate`))
  (bind (_direction _alpha) (`Timeline|AnimChromatic` :!via `PlayFromStart`)
    (:`Update`
      (setmembers `PostProcessSettings` :`StructRef` (`CameraComponent.PostProcessSettings` (`self.Camera`)) :`SceneFringeIntensity` (`KismetMathLibrary.Lerp` 0.0 (`self.MaxChromatic`) _alpha)))))

(event `StartBattle`
  (for (_array_element _array_index) (`self.EnemyTeamLocations`)
    (bind _returnvalue (`|SpawnActorFromClass` (`|GetArrayItem` (`self.EnemyClassesTEMP`) _array_index) (`KismetMathLibrary.MakeTransform` (+ _array_element (`self.SpawnHeightOffset`) (`self.K2_GetActorLocation`))) "AlwaysSpawn" "MultiplyWithRoot" null null))
    (`KismetArrayLibrary.Array_AddUnique` (`self.EnemyTeam`) _returnvalue)
    (`KismetArrayLibrary.Array_AddUnique` (`self.EnemyTeamAlive`) _returnvalue)
    (set `/Game/Blueprints/Battle/BattleChars/BP_BattleChar_BASE.BattleManager` self _returnvalue))
  (for (_array_element_2 _array_index_2) (`self.PartyClassesTEMP`)
    (bind _returnvalue_2 (`|SpawnActorFromClass` _array_element_2 (`KismetMathLibrary.MakeTransform` (+ (`|GetArrayItem` (`self.PartyTeamLocations`) _array_index_2) (`self.SpawnHeightOffset`) (`self.K2_GetActorLocation`)) (`self.PartyTeamRotation`)) "AlwaysSpawn" "MultiplyWithRoot" null null))
    (`KismetArrayLibrary.Array_AddUnique` (`self.PartyTeam`) _returnvalue_2)
    (`KismetArrayLibrary.Array_AddUnique` (`self.PartyTeamAlive`) _returnvalue_2)
    (set `/Game/Blueprints/Battle/BattleChars/BP_BattleChar_BASE.BattleManager` self _returnvalue_2)
    (bind _widgetbattle (message `/Game/Definitions/Interfaces/BPI_UIControl.I_GetWidgetBattle` (`GameplayStatics.GetPlayerController` 0)))
    (bind _aswbp_battle_health_mana (`/Game/UI/Widgets/Battle/WBP_PartyHealthManaPanel.GetCharWidget` (`/Game/UI/Widgets/WBP_Battle.WBP_PartyHealthManaPanel` _widgetbattle) _array_index_2))
    (`/Game/Blueprints/Battle/BattleChars/BP_BattleChar_BASE.AssignBattleHealthManaWidget` _returnvalue_2 _aswbp_battle_health_mana))
  (`self.DecideTurnOrder`)
  (`self.SelectActiveCharacter`)
  (`self.StartCameraSway`)
  (`Controller.Possess` (`GameplayStatics.GetPlayerController` 0) self)
  (`self.StartTurn`))

(event `ConcludeBattle`
  (bind _playerfieldposition (message `/Game/Definitions/Interfaces/BPI_InstanceStorage.I_GetPlayerFieldPosition` (`GameplayStatics.GetGameInstance`)))
  (`GameplayStatics.OpenLevel` (`KismetStringLibrary.Conv_StringToName` (`.FieldLevelName_2_4EFACB7A41468F38A405899DDEDB5CE3` (break `/Game/Definitions/Structs/S_FieldPosition` _playerfieldposition)))))

(event `BattleResult`
  (params (BattleOutcome :type "/Game/Definitions/Enums/E_BattleOutcome Enum" :default "NewEnumerator0"))
  ; Battle Result
  (bind _widgetbattle (message `/Game/Definitions/Interfaces/BPI_UIControl.I_GetWidgetBattle` (`GameplayStatics.GetPlayerController` 0)))
  (`/Game/UI/Widgets/WBP_Battle.CollapseHealthMana` _widgetbattle)
  (switch `/Game/Definitions/Enums/E_BattleOutcome` BattleOutcome
    (:`NewEnumerator0`
      (bind _widgetbattle_2 (message `/Game/Definitions/Interfaces/BPI_UIControl.I_GetWidgetBattle` (`GameplayStatics.GetPlayerController` 0)))
      (`/Game/UI/Widgets/WBP_Battle.ShowBattleResult` _widgetbattle_2)
      (set `self.CanEndBattle` true))
    (:`NewEnumerator1`
      (bind _widgetbattle_3 (message `/Game/Definitions/Interfaces/BPI_UIControl.I_GetWidgetBattle` (`GameplayStatics.GetPlayerController` 0)))
      (`/Game/UI/Widgets/WBP_Battle.ShowNotification` _widgetbattle_3 "Battle Lost" 1.5)
      ;; TEMP. Allow going back  map until there is save system
      (set `self.CanEndBattle` true))
    (:`NewEnumerator2`
      (bind _widgetbattle_4 (message `/Game/Definitions/Interfaces/BPI_UIControl.I_GetWidgetBattle` (`GameplayStatics.GetPlayerController` 0)))
      (`/Game/UI/Widgets/Battle/WBP_ActionMenu.SetActionMenuVisible` (`/Game/UI/Widgets/WBP_Battle.WBP_ActionMenu` _widgetbattle_4) false null)
      (`/Game/UI/Widgets/WBP_Battle.ShowNotification` _widgetbattle_4 "Party Fled" 1.5)
      (`KismetSystemLibrary.RetriggerableDelay` 3.0)
      (`self.ConcludeBattle`))))

(event `AttemptFlee`
  (bind _delayflee (`/Game/Data/DataAssets/GlobalVariables/PDA_GlobalVariables.DelayFlee` (`/Game/Definitions/FunctionLibraries/BPFL_CORE.GetGlobalVariables`)))
  ; Flee
  (if (< (`KismetMathLibrary.RandomFloatInRange` 0.0 100.0) (`/Game/Data/DataAssets/GlobalVariables/PDA_GlobalVariables.FleeChance` (`/Game/Definitions/FunctionLibraries/BPFL_CORE.GetGlobalVariables`)))
    (`self.BattleResult` "NewEnumerator2")
    (else
      (bind _widgetbattle (message `/Game/Definitions/Interfaces/BPI_UIControl.I_GetWidgetBattle` (`GameplayStatics.GetPlayerController` 0)))
      (`/Game/UI/Widgets/WBP_Battle.ShowNotification` _widgetbattle "Flee attempt failed" _delayflee)
      (`/Game/UI/Widgets/Battle/WBP_ActionMenu.SetActionMenuVisible` (`/Game/UI/Widgets/WBP_Battle.WBP_ActionMenu` _widgetbattle) false null)
      (`KismetSystemLibrary.RetriggerableDelay` _delayflee)
      (`self.SkipPartyTurn`)
      (`self.MoveBackFromActive`))))

(event `StartTurn`
  (if (and (not (`KismetArrayLibrary.Array_IsEmpty` (`self.PartyTeamAlive`))) (not (`KismetArrayLibrary.Array_IsEmpty` (`self.EnemyTeamAlive`))))
    (if (`/Game/Blueprints/Battle/BattleChars/BP_BattleChar_BASE.IsPartyMember` (`self.ActiveCharacter`))
      (`self.MoveToActive`)
      (else
        (`self.EnemyTurn`)))))

(event `EnemyTurn`
  (`self.DecideSkill`)
  (`self.DecideTargetPlayer`)
  (`/Game/Blueprints/Battle/BattleChars/BP_BattleChar_BASE.PlayAttackAnim` (`self.ActiveCharacter`) (`self.CurrentSkillData`)))

(event `FinishedTimelineAttackAnim`
  (`/Game/Blueprints/Battle/BattleChars/BP_BattleChar_BASE.ExecuteBattleEffect` (`self.ActiveCharacter`))
  (`KismetSystemLibrary.RetriggerableDelay` (`/Game/Data/DataAssets/GlobalVariables/PDA_GlobalVariables.DelayAfterTimelineAttack` (`/Game/Definitions/FunctionLibraries/BPFL_CORE.GetGlobalVariables`)))
  (`self.ConcludeTurn`))

(event `MoveToActive`
  ;[0.15 0.1362 0.01071 0.5] Move To Active
  (`/Game/UI/Widgets/Battle/WBP_BattleHealthMana.SlideOutAnim` (`/Game/Blueprints/Battle/BattleChars/BP_BattleChar_BASE.WidgetHealthMana` (`self.ActiveCharacter`)))
  (`TimelineComponent.SetPlayRate` (`self.AnimMoveToActive`) (`/Game/Data/DataAssets/GlobalVariables/PDA_GlobalVariables.PlayRateMoveToActive` (`/Game/Definitions/FunctionLibraries/BPFL_CORE.GetGlobalVariables`))) ; TODO: Get rid of magic number
  (bind (_direction _alpha) (`Timeline|AnimMoveToActive` :!via `PlayFromStart`)
    (:`Update`
      (`self.K2_SetActorLocation` (`self.ActiveCharacter`) (`KismetMathLibrary.VLerp` (`/Game/Blueprints/Battle/BattleChars/BP_BattleChar_BASE.SpawnedLocation` (`self.ActiveCharacter`)) (`self.AdjustedActiveLocation`) _alpha) false false))
    (:`Finished`
      (bind _widgetbattle (message `/Game/Definitions/Interfaces/BPI_UIControl.I_GetWidgetBattle` (`GameplayStatics.GetPlayerController` 0)))
      (`/Game/UI/Widgets/Battle/WBP_ActionMenu.SetActionMenuVisible` (`/Game/UI/Widgets/WBP_Battle.WBP_ActionMenu` _widgetbattle) true self))))

(event `MoveBackFromActive`
  ;[0.15 0.1362 0.01071 0.5] Move Back From Active
  (`/Game/UI/Widgets/Battle/WBP_BattleHealthMana.SlideBackAnim` (`/Game/Blueprints/Battle/BattleChars/BP_BattleChar_BASE.WidgetHealthMana` (`self.ActiveCharacter`)))
  (bind _widgetbattle (message `/Game/Definitions/Interfaces/BPI_UIControl.I_GetWidgetBattle` (`GameplayStatics.GetPlayerController` 0)))
  (`/Game/UI/Widgets/Battle/WBP_ActionMenu.SetActionMenuVisible` (`/Game/UI/Widgets/WBP_Battle.WBP_ActionMenu` _widgetbattle) false null)
  (`TimelineComponent.SetPlayRate` (`self.AnimMoveBackFromActive`) (`/Game/Data/DataAssets/GlobalVariables/PDA_GlobalVariables.PlayRateMoveBackActive` (`/Game/Definitions/FunctionLibraries/BPFL_CORE.GetGlobalVariables`))) ; TODO: Get rid of magic number
  (bind (_direction _alpha) (`Timeline|AnimMoveBackFromActive` :!via `PlayFromStart`)
    (:`Update`
      (`self.K2_SetActorLocation` (`self.ActiveCharacter`) (`KismetMathLibrary.VLerp` (`self.AdjustedActiveLocation`) (`/Game/Blueprints/Battle/BattleChars/BP_BattleChar_BASE.SpawnedLocation` (`self.ActiveCharacter`)) _alpha) false false))
    (:`Finished`
      (`KismetSystemLibrary.Delay` 1.0)
      (`self.ConcludeTurn`))))

(event `ConcludeTurn`
  (`/Game/Blueprints/Battle/BattleChars/BP_BattleChar_BASE.HideBattlePortrait` (`self.ActiveCharacter`))
  (`KismetArrayLibrary.Array_Clear` (`self.Targets`))
  (`KismetArrayLibrary.Array_Remove` (`self.TurnOrder`))
  (if (`KismetArrayLibrary.Array_IsEmpty` (`self.TurnOrder`))
    (`self.DecideTurnOrder`)
    (`self.SelectActiveCharacter`)
    (`self.StartTurn`)
    (else
      (`self.SelectActiveCharacter`)
      (`self.StartTurn`))))

(event `EnhancedInput|/Game/Inputs/BattleNav/Actions/IA_BattleNav_Left`
  (params (ActionValue :type Boolean) (ElapsedSeconds :type "Float (double-precision)") (TriggeredSeconds :type "Float (double-precision)") (InputAction :type "InputAction Object Reference" :default "/Game/Inputs/BattleNav/Actions/IA_BattleNav_Left.IA_BattleNav_Left"))
  (:`Started`
    (if (`self.CanBattleNav`)
      (`self.MoveTargetPointer` false))))

(event `EnhancedInput|/Game/Inputs/BattleNav/Actions/IA_BattleNav_Right`
  (params (ActionValue :type Boolean) (ElapsedSeconds :type "Float (double-precision)") (TriggeredSeconds :type "Float (double-precision)") (InputAction :type "InputAction Object Reference" :default "/Game/Inputs/BattleNav/Actions/IA_BattleNav_Right.IA_BattleNav_Right"))
  (:`Started`
    (if (`self.CanBattleNav`)
      (`self.MoveTargetPointer` true))))

(event `EnhancedInput|/Game/Inputs/BattleNav/Actions/IA_BattleNav_Accept`
  (params (ActionValue :type Boolean) (ElapsedSeconds :type "Float (double-precision)") (TriggeredSeconds :type "Float (double-precision)") (InputAction :type "InputAction Object Reference" :default "/Game/Inputs/BattleNav/Actions/IA_BattleNav_Accept.IA_BattleNav_Accept"))
  (:`Started`
    (if (`self.CanEndBattle`)
      (`self.ConcludeBattle`)
      (elif (`self.CanBattleNav`)
        (`/Game/Blueprints/Battle/BattleChars/BP_BattleChar_BASE.PlayAttackAnim` (`self.ActiveCharacter`) (`self.CurrentSkillData`))
        (`self.EndTargetPickMode`)))))

(event `EnhancedInput|/Game/Inputs/BattleNav/Actions/IA_BattleNav_Back`
  (params (ActionValue :type Boolean) (ElapsedSeconds :type "Float (double-precision)") (TriggeredSeconds :type "Float (double-precision)") (InputAction :type "InputAction Object Reference" :default "/Game/Inputs/BattleNav/Actions/IA_BattleNav_Back.IA_BattleNav_Back"))
  (:`Started`
    (if (`self.CanBattleNav`)
      (`self.EndTargetPickMode`)
      (bind _widgetbattle (message `/Game/Definitions/Interfaces/BPI_UIControl.I_GetWidgetBattle` (`GameplayStatics.GetPlayerController` 0)))
      (`/Game/UI/Widgets/Battle/WBP_ActionMenu.SetActionMenuVisible` (`/Game/UI/Widgets/WBP_Battle.WBP_ActionMenu` _widgetbattle) true self))))

(fn `ApplyBattleEffect`
  (params (InstigatorStats :type "/Game/Blueprints/Components/AC_BattleStats Object Reference"))
  (for _array_element (`self.Targets`)
    (`/Game/Blueprints/Battle/BattleChars/BP_BattleChar_BASE.ReceiveBattleEffect` _array_element (`local.InstigatorStats`) (`self.CurrentSkillData`)))
  (bind _widgetbattle (message `/Game/Definitions/Interfaces/BPI_UIControl.I_GetWidgetBattle` (`GameplayStatics.GetPlayerController` 0)))
  (`/Game/UI/Widgets/WBP_Battle.ShowNotification` _widgetbattle (`/Game/Data/DataAssets/SkillData/PDA_SkillData.SkillName` (`self.CurrentSkillData`)) 1.5)
  (`self.PlayChromaticPulse`))

(fn `DecideSkill`
  (set `self.CurrentSkillData` (`/Game/Data/DataAssets/BattleCharData/PDA_BattleCharData.BasicAttackData` (`/Game/Blueprints/Battle/BattleChars/BP_BattleChar_BASE.BattleCharData` (`self.ActiveCharacter`)))))

(fn `DecideTargetPlayer`
  (switch `/Game/Definitions/Enums/E_TargetStyle` (`/Game/Data/DataAssets/SkillData/PDA_SkillData.TargetStyle` (`self.CurrentSkillData`))
    (:`NewEnumerator0`
      (`KismetArrayLibrary.Array_Set` (`self.Targets`) 0 (`KismetArrayLibrary.Array_Random` (`self.PartyTeamAlive`)) true))
    (:`NewEnumerator1`
      (set `self.Targets` (`self.PartyTeamAlive`)))))

(fn `DecideTurnOrder`
  (`KismetArrayLibrary.Array_Clear` (`self.TurnOrder`))
  (`KismetArrayLibrary.Array_Append` (`self.TurnOrder`) (`self.PartyTeamAlive`))
  (`KismetArrayLibrary.Array_Append` (`self.TurnOrder`) (`self.EnemyTeamAlive`))
  (bind _widgetbattle (message `/Game/Definitions/Interfaces/BPI_UIControl.I_GetWidgetBattle` (`GameplayStatics.GetPlayerController` 0)))
  (`/Game/UI/Widgets/Battle/WBP_TurnOrder.ReplaceTurnOrder` (`/Game/UI/Widgets/WBP_Battle.WBP_TurnOrder` _widgetbattle) (`self.TurnOrder`)))

(fn `EndTargetPickMode`
  (for _array_element (`self.Targets`)
    (`/Game/Blueprints/Battle/BattleChars/BP_BattleChar_BASE.SetPointerVisibility` _array_element false))
  (set `self.TargetIndex` 0)
  (set `self.CanBattleNav` false))

(fn `GetTargetTeam`
  (returns (ReturnValue :type "Array of /Game/Blueprints/Battle/BattleChars/BP_BattleChar_BASE Object Reference"))
  (return (select `/Game/Definitions/Enums/E_TargetGroup` (`/Game/Data/DataAssets/SkillData/PDA_SkillData.TargetGroup` (`self.CurrentSkillData`)) :`NewEnumerator0` (`self.EnemyTeamAlive`) :`NewEnumerator1` (`self.PartyTeamAlive`))))

(fn `MoveTargetPointer`
  (params (MoveRight :type Boolean))
  (if (`|EnumEquality` (`/Game/Data/DataAssets/SkillData/PDA_SkillData.TargetStyle` (`self.CurrentSkillData`)) "NewEnumerator0")
    (`/Game/Blueprints/Battle/BattleChars/BP_BattleChar_BASE.SetPointerVisibility` (`|GetArrayItem` (`self.Targets`)) false)
    (if (`local.MoveRight`)
      (`/Engine/EditorBlueprintResources/StandardMacros.IncrementInt` (`self.TargetIndex`)
        (:`  `
          _))
      (else
        (`/Engine/EditorBlueprintResources/StandardMacros.DecrementInt` (`self.TargetIndex`)
          (:`  `
            _))))
    (set `self.TargetIndex` (`KismetMathLibrary.Clamp` (`self.TargetIndex`) 0 (`KismetArrayLibrary.Array_LastIndex` (`self.GetTargetTeam`))))
    (`KismetArrayLibrary.Array_Set` (`self.Targets`) 0 (`|GetArrayItem` (`self.GetTargetTeam`) (`self.TargetIndex`)) true)
    (`/Game/Blueprints/Battle/BattleChars/BP_BattleChar_BASE.SetPointerVisibility` (`|GetArrayItem` (`self.Targets`)) true)))

(fn `RemoveFromTurnOrder`
  (params (CharToRemove :type "/Game/Blueprints/Battle/BattleChars/BP_BattleChar_BASE Object Reference"))
  (`KismetArrayLibrary.Array_RemoveItem` (`self.TurnOrder`) CharToRemove))

(fn `SelectActiveCharacter`
  (set `self.ActiveCharacter` (`|GetArrayItem` (`self.TurnOrder`)))
  (`/Game/Blueprints/Battle/BattleChars/BP_BattleChar_BASE.SetDefending` (`self.ActiveCharacter`) false))

(fn `SkipPartyTurn`
  (for _array_element (`self.PartyTeamAlive`)
    (`KismetArrayLibrary.Array_RemoveItem` (`self.TurnOrder`) _array_element)
    (`/Game/Blueprints/Battle/BattleChars/BP_BattleChar_BASE.HideBattlePortrait` _array_element)))

(fn `StartDefending`
  (`/Game/Blueprints/Battle/BattleChars/BP_BattleChar_BASE.SetDefending` (`self.ActiveCharacter`) true)
  (`self.MoveBackFromActive`))

(fn `StartTargetPickMode`
  (params (SkillIndex :type Integer))
  (bind _skilldata (`/Game/Blueprints/Battle/BattleChars/BP_BattleChar_BASE.GetSkillByIndex` (`self.ActiveCharacter`) (`local.SkillIndex`)))
  (set `self.CurrentSkillData` _skilldata)
  (`KismetArrayLibrary.Array_Clear` (`self.Targets`))
  (`|ExecutionSequence`
    (:`then_0`
      (switch `/Game/Definitions/Enums/E_TargetStyle` (`/Game/Data/DataAssets/SkillData/PDA_SkillData.TargetStyle` (`self.CurrentSkillData`))
        (:`NewEnumerator0`
          (`KismetArrayLibrary.Array_Set` (`self.Targets`) 0 (`|GetArrayItem` (`self.GetTargetTeam`)) true))
        (:`NewEnumerator1`
          (set `self.Targets` (`self.GetTargetTeam`)))))
    (:`then_1`
      (for _array_element (`self.Targets`)
        (`/Game/Blueprints/Battle/BattleChars/BP_BattleChar_BASE.SetPointerVisibility` _array_element true)))
    (:`then_2`
      (bind _widgetbattle (message `/Game/Definitions/Interfaces/BPI_UIControl.I_GetWidgetBattle` (`GameplayStatics.GetPlayerController` 0)))
      (`/Game/UI/Widgets/Battle/WBP_ActionMenu.SetActionMenuVisible` (`/Game/UI/Widgets/WBP_Battle.WBP_ActionMenu` _widgetbattle) false null)
      (message `/Game/Definitions/Interfaces/BPI_UIControl.I_DeactivateUIControls` (`GameplayStatics.GetPlayerController` 0))
      (set `self.CanBattleNav` true))))

(fn `UpdateTeamAlive`
  (params (CharToRemove :type "/Game/Blueprints/Battle/BattleChars/BP_BattleChar_BASE Object Reference"))
  (`self.RemoveFromTurnOrder` (`local.CharToRemove`))
  (if (`/Game/Blueprints/Battle/BattleChars/BP_BattleChar_BASE.IsPartyMember` (`local.CharToRemove`))
    (`KismetArrayLibrary.Array_RemoveItem` (`self.PartyTeamAlive`) (`local.CharToRemove`))
    (if (`KismetArrayLibrary.Array_IsEmpty` (`self.PartyTeamAlive`))
      (`self.BattleResult` "NewEnumerator1"))
    (else
      (`KismetArrayLibrary.Array_RemoveItem` (`self.EnemyTeamAlive`) (`local.CharToRemove`))
      (if (`KismetArrayLibrary.Array_IsEmpty` (`self.EnemyTeamAlive`))
        (`self.BattleResult` "NewEnumerator0")))))

(fn `UserConstructionScript`)