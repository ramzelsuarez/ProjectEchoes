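; BP_NPCJoin is a field NPC that joins the player's party once its conversation ends.
; When the conversation lock is released, it messages the player pawn through an interface to spawn a single member from its PartyMember data at its transform, then destroys itself.
; Its speaker name comes from that member's battle character display name, falling back to the parent's name when the data is invalid.
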(event `/Game/Definitions/Interfaces/BPI_DialogueControl.I_SetCoversationLock`
  (params (SetLocked :type Boolean))
  (`parent.I_SetCoversationLock` SetLocked)
  (if (not SetLocked)
    (message `/Game/Definitions/Interfaces/BPI_PartyControl.I_SpawnSingleMember` (`GameplayStatics.GetPlayerPawn` 0) (`self.GetTransform`) (`self.PartyMember`))
    (`self.K2_DestroyActor`)))

(fn `I_GetSpeakerName`
  (returns (SpeakerName :type Text))
  (bind _partymember (`self.PartyMember`)
    (:`then`
      (return (`/Game/Data/DataAssets/BattleCharData/PDA_BattleCharData.DisplayName` (`/Game/Data/DataAssets/PartyMemberData/PDA_PartyMemberData.BattleCharData` _partymember))))
    (:`else`
      (bind _speakername (`parent.I_GetSpeakerName`))
      (return _speakername))))

(fn `UserConstructionScript`
  (`parent.UserConstructionScript`))