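; BP_FieldPlayer is the player character or pawn for the field part of the game.
; On BeginPlay it has the player controller create the field widget through interface messages, then plays the widget's transition open animation.
; Possession adds the field Enhanced Input mapping context, whose move action drives movement along fixed world X and Y axes.
; StoreFieldPositionOnInstance passes the actor transform to the GameInstance through an interface message.
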(event `self.ReceiveBeginPlay`
  (`parent.ReceiveBeginPlay`)
  (message `/Game/Definitions/Interfaces/BPI_UIControl.I_InitWidgetField` (`GameplayStatics.GetPlayerController` 0))
  (bind _widgetfield (message `/Game/Definitions/Interfaces/BPI_UIControl.I_GetWidgetField` (`GameplayStatics.GetPlayerController` 0)))
  (`/Game/UI/Widgets/WBP_Transition.PlayOpenAnim` (`/Game/UI/Widgets/WBP_Field.WBP_Transition` _widgetfield)))

(event `self.ReceivePossessed`
  (params (NewController :type "Controller Object Reference"))
  (`parent.ReceivePossessed` NewController)
  (bind _asplayer_controller (cast `PlayerController` (`self.GetController`)))
  (`EnhancedInputSubsystemInterface.AddMappingContext` (pcsubsystem `EnhancedInputLocalPlayerSubsystem` _asplayer_controller) "/Game/Inputs/Field/IMC_Field.IMC_Field" 0 (struct)))

(event `EnhancedInput|/Game/Inputs/Field/Actions/IA_Move`
  (params (ActionValue :type "Vector2D Structure") (ElapsedSeconds :type "Float (double-precision)") (TriggeredSeconds :type "Float (double-precision)") (InputAction :type "InputAction Object Reference" :default "/Game/Inputs/Field/Actions/IA_Move.IA_Move"))
  (bind (_x _y) (`KismetMathLibrary.BreakVector2D` ActionValue))
  (:`Triggered`
    (`self.AddMovementInput` (1.0 0.0 0.0) _x)
    (`self.AddMovementInput` (0.0 1.0 0.0) _y)))

(fn `StoreFieldPositionOnInstance`
  (message `/Game/Definitions/Interfaces/BPI_InstanceStorage.I_StoreFieldPosition` (`GameplayStatics.GetGameInstance`) (`self.GetTransform`)))

(fn `UserConstructionScript`
  (`parent.UserConstructionScript`))