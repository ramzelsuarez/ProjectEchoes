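; BP_Chest is an interactable field chest that gives the player a one-time item reward.
; Interacting calls Open, which sets IsOpened, plays the open animation and sends the Reward item to the GameInstance inventory through an interface.
; It then shows a "Received" notification on the field widget and triggers its ACIdentifier component's ID.
; The can-interact check returns false once opened.
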(event `self.ReceiveBeginPlay`)

(event `/Game/Definitions/Interfaces/BPI_Interactable.I_Interact`
  (`self.Open`))

(fn `I_CanInteract`
  (returns (CanInteract :type Boolean))
  (return (not (`self.IsOpened`))))

(fn `Open`
  (bind (_itemdata _amount) (break `/Game/Definitions/Structs/S_ItemStack` (`self.Reward`)))
  (if (not (`self.IsOpened`))
    (set `self.IsOpened` true)
    (`SkeletalMeshComponent.PlayAnimation` (`self.Chest`) "/Game/Art/Environment/Props/Meshes/Chest/Chest_Wood_Anim_Chest_Armature_Chest_Open.Chest_Wood_Anim_Chest_Armature_Chest_Open" false)
    (message `/Game/Definitions/Interfaces/BPI_InstanceStorage.I_AddItemToInventory` (`GameplayStatics.GetGameInstance`) _itemdata _amount)
    (bind _widgetfield (message `/Game/Definitions/Interfaces/BPI_UIControl.I_GetWidgetField` (`GameplayStatics.GetPlayerController` 0)))
    (`/Game/UI/Widgets/WBP_Field.ShowNotification` _widgetfield (`|FormatText` "Received: {ItemName} x{ItemAmount}" (`/Game/Data/DataAssets/ItemData/PDA_ItemData.ItemName` _itemdata) _amount) 3.0)
    (`/Game/Blueprints/Components/AC_Identifier.TriggerID` (`self.AC_Identifier`))))

(fn `UserConstructionScript`)